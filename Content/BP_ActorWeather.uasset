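; BP_ActorWeather is the startup actor for a city weather lookup interface.
; On BeginPlay it shows the mouse cursor, creates BP_MainWidget, passes itself to it, sets Russian usage instructions and has the widget fill its scroll box from a database.
; It also disables move and look input and forces a small fixed-size windowed resolution through game user settings and a console command.
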(event `self.ReceiveBeginPlay`
  (bind _returnvalue (`GameplayStatics.GetPlayerController` 0))
  (bind _wvarmainwidget (`self.WVarMainWidget`))
  (set `PlayerController.bShowMouseCursor` true _returnvalue)
  (bind _returnvalue_2 (`|CreateWidget` "/Game/BP_MainWidget.BP_MainWidget_C" _returnvalue))
  (bind _output_get (set `self.WVarMainWidget` _returnvalue_2))
  (`UserWidget.AddToViewport` _wvarmainwidget 0)
  (set `/Game/BP_MainWidget.WVarWeatherActor` self _wvarmainwidget)
  (`TextBlock.SetText` (`/Game/BP_MainWidget.DetailedWeatherText` _wvarmainwidget) "Введите название города для получения данные о погоде.  \nЕсли город найден, его можно Добавить в список. \nДля обновления информации города из списка, \nнажать кнопку справа от имени города.")
  (`/Game/BP_MainWidget.BP_FillScrollBoxFromDB` _output_get)
  (`Controller.SetIgnoreMoveInput` _returnvalue true)
  (`Controller.SetIgnoreLookInput` _returnvalue true)
  (bind _returnvalue_3 (`GameUserSettings.GetGameUserSettings`))
  (`GameUserSettings.SetFullscreenMode` _returnvalue_3 "Windowed")
  (`GameUserSettings.SetScreenResolution` _returnvalue_3 (make `IntPoint` 1136 640))
  (`KismetSystemLibrary.ExecuteConsoleCommand` "r.SetRes 1136x640" null))

(fn `UserConstructionScript`)